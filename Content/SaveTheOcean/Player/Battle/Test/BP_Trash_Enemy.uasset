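; Test trash enemy actor for battle that loses HP when another actor's overlap with it ends.
; On end overlap it casts the other actor, then calls BeBeaten if the Beatend flag is set, or prints "Miss" otherwise.
; BeBeaten subtracts the cast actor's Damage from HP and prints the result, with no death handling.
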(event Custom|BeBeaten
  (bind _output_get (Variables|Default|SetHP (- (Variables|Default|GetHP) (Variables|Default|GetDamage (stale Collision|EventActorEndOverlap _asbp_main_player)))))
  (Development|PrintString (Utilities|String|ToString(Float) _output_get) true true "(R=0.000000,G=1.000000,B=0.277501,A=1.000000)"))

(event EventBeginPlay)

(event EventTick
  (params (DeltaSeconds :type Float%20%28single-precision%29)))

(event Collision|EventActorEndOverlap
  (params (OtherActor :type Actor%20Object%20Reference))
  (bind _asbp_main_player (Utilities|Casting|CastTo OtherActor))
  (if (Variables|Default|GetBeatend?)
    (CallFunction|BeBeaten)
    (else
      (Development|PrintString "Miss"))))

(fn ConstructionScript)