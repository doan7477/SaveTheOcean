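; BP_MainPlayer is the player character for SaveTheOcean, playing a scripted walk, attack and return routine when play begins.
; BeginPlay calls Attack whether or not AttackStatus is set, and any actor overlap sets IsEnemy, which only gates a debug print.
; Attack chains timelines and a delay to move and turn the actor, while parallel timelines drive Speed on the BP_CharacterMovement anim instance.
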(event Custom|Attack
  ;[1 1 1] #3 Attack
  (bind _asbp_character_movement (Utilities|Casting|CastToBP_CharacterMovement (Components|SkeletalMesh|GetAnimInstance (Variables|Default|GetSkeletalMesh))))
  (Utilities|FlowControl|Sequence
    (:then_0
      (bind _behavior_1 (Timeline|Behavior PlayFromStart)
        (:Update
          (Variables|/Game/SaveTheOcean/Player/Character_Player/BP_CharacterMovement.BP_CharacterMovement_C|SetSpeed _asbp_character_movement _behavior_1))))
    (:then_1
      (bind _movement (Timeline|Move_1 PlayFromStart)
        (:Update
          (Class|Actor|AddActorLocalTransform (Math|Transform|MakeTransform (Math|Vector|MakeVector 0.0 _movement 0.0) "0, 0, 0" "1,1,1") false false))
        (:Finished
          (bind _behavior_1_2 (Timeline|Attack_1 PlayFromStart)
            (:Update
              (Variables|/Game/SaveTheOcean/Player/Character_Player/BP_CharacterMovement.BP_CharacterMovement_C|SetSpeed _asbp_character_movement _behavior_1_2))
            (:Finished
              (Utilities|FlowControl|Delay 2.8)
              (if (Variables|Default|GetIsEnemy)
                (Development|PrintString "Attack"))
              (Utilities|FlowControl|Sequence
                (:then_0
                  (bind _rotation (Timeline|Turn_1 PlayFromStart)
                    (:Update
                      (Transformation|AddActorLocalRotation (Math|Rotator|MakeRotator 0.0 0.0 _rotation) false false))))
                (:then_1
                  (Utilities|FlowControl|Sequence
                    (:then_0
                      (bind _behavior_1_3 (Timeline|WalkAgain PlayFromStart)
                        (:Update
                          (Variables|/Game/SaveTheOcean/Player/Character_Player/BP_CharacterMovement.BP_CharacterMovement_C|SetSpeed _asbp_character_movement _behavior_1_3))))
                    (:then_1
                      (bind _movement_2 (Timeline|Move_2 PlayFromStart)
                        (:Update
                          (Class|Actor|AddActorLocalTransform (Math|Transform|MakeTransform (Math|Vector|MakeVector 0.0 _movement_2 0.0) "0, 0, 0" "1,1,1") false false))
                        (:Finished
                          (Utilities|FlowControl|Sequence
                            (:then_0
                              (bind _behavior_1_4 (Timeline|BreathAgain PlayFromStart)
                                (:Update
                                  (Variables|/Game/SaveTheOcean/Player/Character_Player/BP_CharacterMovement.BP_CharacterMovement_C|SetSpeed _asbp_character_movement _behavior_1_4))))
                            (:then_1
                              (bind _rotation_2 (Timeline|Turn_2 PlayFromStart)
                                (:Update
                                  (Transformation|AddActorLocalRotation (Math|Rotator|MakeRotator 0.0 0.0 _rotation_2) false false))))))))))))))))))

(event EventBeginPlay
  ;[1 1 1] #1 Check the Beat Boolean
  (if (Variables|Default|GetAttackStatus)
    (Development|PrintString "GoAttack")
    (CallFunction|Attack)
    (else
      (CallFunction|Attack))))

(event EventTick
  (params (DeltaSeconds :type Float%20%28single-precision%29)))

(event Collision|EventActorBeginOverlap
  (params (OtherActor :type Actor%20Object%20Reference))
  ;[1 1 1] #2 Check the Trash Boolean
  (Variables|Default|SetIsEnemy true)
  (Development|PrintString (Utilities|GetDisplayName OtherActor) true true "(R=1.000000,G=0.000000,B=0.058156,A=1.000000)"))

(fn ConstructionScript)