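; Player character for turn-based battles, with attack, heal, risk attack, kick, buff, hit, victory and runaway actions.
; BeginPlay copies stats from PlayerInfo and finds the enemy actor named in GameInstance save data; Tick updates a target point before it.
; Actions set an animation State and use delays and timelines to move, turn or raise the character.
; Attacks call the enemy's Hit; VictoryCheck triggers victory and level-up checks when enemy health runs out.
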(event Custom|VIctory
  ;[1 1 1] #3 Victory (IncludeLvUpFunction)
  (Variables|Default|SetState "NewEnumerator4")
  (if (>= (+ (Variables|Default|GetExperience%20Point%20EXP) (Variables|/Game/SaveTheOcean/Enemy/BP_Parent_Enemy.BP_Parent_Enemy_C|GetEx (Variables|Default|GetEnemy))) (Variables|Default|GetLv_Up_EXP)) ; 레벨업 여부
    (Variables|Default|SetLv_Up_EXP (+ (Variables|Default|GetLv_Up_EXP) 1.0)) ; 레벨업에 따른 기준 경험치 상향조정
    (Variables|Default|SetPlayer%20Info%20Player%20Level (+ (Variables|Default|GetPlayer%20Info%20Player%20Level) 1))
    (Development|PrintString "Congratulations! You've gotten level up!"))
  (Utilities|FlowControl|Delay 2.0)
  (Variables|Default|SetState "NewEnumerator1"))

(event Custom|Attack
  (bind _startpoint (Variables|Default|GetStartPoint))
  (bind _target_vector (Variables|Default|GetTarget_Vector))
  ;[1 1 1] #1 Attack
  ;;[1 1 1] 캐릭터 전진
  (Variables|Default|SetState "NewEnumerator0")
  (bind _speed (Timeline|MoveForward PlayFromStart)
    (:Update
      (Transformation|SetActorLocation (+ (* (- (Variables|Default|GetTarget_Vector) _startpoint) _speed) _startpoint) false false))
    (:Finished
      ;;[1 1 1] 캐릭터 공격
      (Variables|Default|SetState "NewEnumerator2")
      (Utilities|FlowControl|Delay 1.2) ; 사운드넣기
      (Default|Hit (Variables|Default|GetEnemy) (Variables|Default|GetOffense%20Power%20AD)) ; Call the Enemy Hit Function
      (Utilities|FlowControl|Delay 1.4) ; 사운드넣기
      (Utilities|FlowControl|Sequence
        (:then_0
          ;;[1 1 1] 원래 자리로 돌아가기
          (Variables|Default|SetState "NewEnumerator0")
          (bind _speed_2 (Timeline|Return PlayFromStart)
            (:Update
              (Transformation|SetActorLocation (+ (* (- (Variables|Default|GetStartPoint) _target_vector) _speed_2) _target_vector) false false))
            (:Finished
              (Variables|Default|SetState "NewEnumerator1")
              (Variables|Default|SetOffense%20Power%20AD 1e+01) ; 공격력 원상회복
              ;;[1 1 1] 캐릭터 회전
              (Variables|Default|SetReturn%20Value%20Z%20%28Yaw%29 (.yaw (Transformation|GetActorRotation)) :!label _label)
              (bind _rotation (Timeline|Turn_Physic PlayFromStart)
                (:Update
                  (Transformation|SetActorRotation (Math|Rotator|MakeRotator 0.0 0.0 (Math|Float|Lerp (Variables|Default|GetReturn%20Value%20Z%20%28Yaw%29) (+ (Variables|Default|GetReturn%20Value%20Z%20%28Yaw%29) 1.8e+02) _rotation))))
                (:Finished)))))
        (:then_1
          (goto _label))))))

(event Custom|Kick
  (bind _target_vector (Variables|Default|GetTarget_Vector))
  (bind _startpoint (Variables|Default|GetStartPoint))
  ;[1 1 1] #5.3 Skill : Kick
  (if (>= (Variables|Default|GetMana%20Points%20MP) 4e+01)
    ;;[1 1 1] 기본공격 대비 10% 증가된 데미지로 강타
    (Variables|Default|SetOffense%20Power%20AD (* (Variables|Default|GetOffense%20Power%20AD) 1.1))
    ;;[1 1 1] 캐릭터 전진
    (Variables|Default|SetState "NewEnumerator0")
    (bind _speed (Timeline|타임라인_3 PlayFromStart)
      (:Update
        (Transformation|SetActorLocation (+ (* (- (Variables|Default|GetTarget_Vector) _startpoint) _speed) _startpoint) false false))
      (:Finished
        ;;[1 1 1] 캐릭터 공격
        (Variables|Default|SetState "NewEnumerator7")
        (Utilities|FlowControl|Delay 1.4) ; 사운드넣기
        (Default|Hit (Variables|Default|GetEnemy) 0.0) ; Call the Enemy Hit Function
        (Utilities|FlowControl|Delay 0.6) ; 사운드넣기
        ;;;[1 1 1] 공격력 원상복귀
        (Variables|Default|SetOffense%20Power%20AD (/ (Variables|Default|GetOffense%20Power%20AD) 1.1))
        (Utilities|FlowControl|Sequence
          (:then_0
            (Variables|Default|SetState "NewEnumerator0")
            (bind _speed_2 (Timeline|타임라인_5 PlayFromStart)
              (:Update
                (Transformation|SetActorLocation (+ (* (- (Variables|Default|GetStartPoint) _target_vector) _speed_2) _target_vector) false false))
              (:Finished
                (Variables|Default|SetState "NewEnumerator1")
                ;;[1 1 1] 캐릭터 회전
                (Variables|Default|SetReturn%20Value%20Z%20%28Yaw%29 (.yaw (Transformation|GetActorRotation)) :!label _label)
                (bind _rotation (Timeline|타임라인_4 PlayFromStart)
                  (:Update
                    (Transformation|SetActorRotation (Math|Rotator|MakeRotator 0.0 0.0 (Math|Float|Lerp (Variables|Default|GetReturn%20Value%20Z%20%28Yaw%29) (+ (Variables|Default|GetReturn%20Value%20Z%20%28Yaw%29) 1.8e+02) _rotation))))))))
          (:then_1
            (goto _label)))))
    (else
      (Development|PrintString "You've not enogh MP."))))

(event Custom|Heal
  ;[1 1 1] #5.1 Skill : Heal
  (if (> (Variables|Default|GetHealth%20Points%20HP) 0.0) ; IsPlayerAlive?
    (Variables|Default|SetState "NewEnumerator5")
    (Variables|Default|SetHealth%20Points%20HP (+ (Variables|Default|GetHealth%20Points%20HP) 1e+02))
    (Development|PrintString (Utilities|String|ToString(Float) (Variables|Default|GetHealth%20Points%20HP)))
    (Utilities|FlowControl|Delay 2.8)
    (Variables|Default|SetState "NewEnumerator1")
    (else
      (Development|PrintString (Utilities|String|ToString(Float) (Variables|Default|GetHealth%20Points%20HP)) true true "(R=0.000000,G=1.000000,B=0.184247,A=1.000000)"))))

(event Custom|Hit
  (params (Damage :type Float%20%28single-precision%29))
  ;[1 1 1] #2 Hit
  (Variables|Default|SetState "NewEnumerator3")
  (Variables|Default|SetHealth%20Points%20HP (- (Variables|Default|GetHealth%20Points%20HP) Damage))
  (Utilities|FlowControl|Delay 1.5)
  (if (> (Variables|Default|GetHealth%20Points%20HP) 0.0) ; IsPlayerAlive?
    (if (Variables|Default|GetReadytoUse?)
      (Variables|Default|SetState "NewEnumerator10")
      (else
        (Variables|Default|SetState "NewEnumerator1")))
    (else
      (Development|PrintString "You're dead" true true "(R=0.000000,G=1.000000,B=0.184247,A=1.000000)"))))

(event Custom|Stay
  ;[1 1 1] #4 Stay
  (Variables|Default|SetState "NewEnumerator1"))

(event Custom|Buff
  ;[1 1 1] #5.4 Skill : Power UP (Buff)
  (if (>= (Variables|Default|GetMana%20Points%20MP) 4e+01)
    (Variables|Default|SetOffense%20Power%20AD (* (Variables|Default|GetOffense%20Power%20AD) 1.2)) ; 공격사용시까지 공격력 20% 증가
    (Variables|Default|SetState "NewEnumerator8")
    ;;[1 1 1] Z값 이동
    (bind _up (Timeline|타임라인_1 PlayFromStart)
      (:Update
        (Transformation|SetRelativeLocation (Variables|Character|GetMesh) (Math|Vector|MakeVector 0.0 0.0 (Math|Float|Lerp -9e+01 5e+01 _up)) false false))
      (:Finished
        (Variables|Default|SetState "NewEnumerator9")
        (Development|PrintString "Offensive Buff is Activating.")
        (Utilities|FlowControl|Delay 2.0)
        (Variables|Default|SetState "NewEnumerator1")))
    (else
      (Development|PrintString "You've not enogh MP."))))

(event Custom|Runaway
  ;[1 1 1] #6 RunAway
  (if (> (Variables|Default|GetHealth%20Points%20HP) 0.0)
    ;;[1 1 1] 레벨 확정되면 이동할 공간으로 플레이어 전송
    (Transformation|SetActorLocation "9999.000000,9999.000000,9999.000000" false false)))

(event Custom|Skill_RiskAttack
  ;[1 1 1] #5.2 Skill : RiskAttack
  (if (>= (Variables|Default|GetMana%20Points%20MP) 4e+01)
    (if (Variables|Default|GetReadytoUse?)
      (Utilities|FlowControl|Delay 0.5) ; 오작동 예방 쿠션
      ;;[1 1 1] 캐릭터 공격
      (Variables|Default|SetState "NewEnumerator11")
      (Utilities|FlowControl|Sequence ; 공격 및 Idle 노드 실행
        (:then_0
          (Utilities|FlowControl|Delay 1.6) ; 사운드넣기
          (Utilities|FlowControl|Sequence ; Hit & Z값 보정 실행
            (:then_0
              (Default|Hit (Variables|Default|GetEnemy) 0.0) ; Call the Enemy Hit Function
              (Variables|Default|SetReadytoUse? false) ; 끈기 상태였을 경우 해제
              (Variables|Default|SetOffense%20Power%20AD 1e+01) ; 공격력 원상회복
            )
            (:then_1
              ;;[1 0 0.851] 타격시 Z값보정
              (Variables|Default|SetMeshLocation_Z -75.0)
              (bind _up (Timeline|타임라인_0 PlayFromStart)
                (:Update
                  (Transformation|SetRelativeLocation (Variables|Character|GetMesh) (Math|Vector|MakeVector 0.0 0.0 (Math|Float|Lerp -88.0 (Variables|Default|GetMeshLocation_Z) _up)) false false))
                (:Finished
                  ;;[1 1 1] 캐릭터 파워 세이빙
                  ;;;[1 0 0.851] Idle 또는 Crouch시 Z값 보정
                  (bind _up_2 (Timeline|MoveUp ReverseFromEnd)
                    (:Update
                      (Transformation|SetRelativeLocation (Variables|Character|GetMesh) (Math|Vector|MakeVector 0.0 0.0 (Math|Float|Lerp -9e+01 (Variables|Default|GetMeshLocation_Z) _up_2)) false false))
                    (:Finished
                      (Variables|Default|SetOffense%20Power%20AD (* (Variables|Default|GetOffense%20Power%20AD) 2.0)) ; 공격사용시까지 공격력 2배 증가
                      (Development|PrintString "You can use the Magic Attack next turn."))))))))
        (:then_1
          ;;;[0 0.1203 1] 자연스러운 애니메이션에는 2sec 필요
          (Utilities|FlowControl|Delay 2.0)
          (Variables|Default|SetState "NewEnumerator1")))
      (else
        (Variables|Default|SetReadytoUse? true)
        (Variables|Default|SetState "NewEnumerator6")
        (Utilities|FlowControl|Delay 1.4) ; 사운드넣기
        (Utilities|FlowControl|Sequence
          (:then_0
            (Variables|Default|SetMeshLocation_Z -88.0)
            (Timeline|MoveUp PlayFromStart))
          (:then_1
            (Variables|Default|SetState "NewEnumerator10")))))
    (else
      (Development|PrintString "You've not enogh MP."))))

(event EventBeginPlay
  (bind _playerinfo (Variables|Default|GetPlayerInfo))
  (bind (_playerlevel _healthpoints_hp _manapoints_mp _experiencepoint_exp _offensepower_ad) (Utilities|Struct|BreakBP_PlayerInfo _playerinfo))
  ;[1 1 1] #0 Set the Player Info
  (Variables|Default|SetPlayer%20Info%20Player%20Level _playerlevel)
  (Variables|Default|SetHealth%20Points%20HP _healthpoints_hp)
  (Variables|Default|SetMana%20Points%20MP _manapoints_mp)
  (Variables|Default|SetExperience%20Point%20EXP _experiencepoint_exp)
  (Variables|Default|SetOffense%20Power%20AD _offensepower_ad)
  (Variables|Default|SetStartPoint (Transformation|GetActorLocation))
  ;[1 1 1] Enemyname
  (bind _assave_the_ocean_game_instance (Utilities|Casting|CastToSaveTheOceanGameInstance (Game|GetGameInstance)))
  (switch Utilities|FlowControl|Switch|SwitchonEnemyName (Variables|/Game/SaveTheOcean/Core/SaveGameBP.SaveGameBP_C|GetEnemyName (Variables|/Game/SaveTheOcean/Core/SaveTheOceanGameInstance.SaveTheOceanGameInstance_C|GetSaveData _assave_the_ocean_game_instance))
    (:NewEnumerator0
      (bind _returnvalue (Actor|GetActorOfClass "/Game/SaveTheOcean/Enemy/BP_child_TrashMan.BP_child_TrashMan_C"))
      (Variables|Default|SetEnemy _returnvalue))
    (:NewEnumerator1
      (bind _returnvalue_2 (Actor|GetActorOfClass "/Game/SaveTheOcean/Enemy/BP_child_Drum.BP_Child_Drum_C"))
      (Variables|Default|SetEnemy _returnvalue_2))
    (:NewEnumerator2
      (bind _returnvalue_3 (Actor|GetActorOfClass "/Game/SaveTheOcean/Enemy/BP_child_Boss.BP_child_Boss_C"))
      (Variables|Default|SetEnemy _returnvalue_3))))

(event EventTick
  (params (DeltaSeconds :type Float%20%28single-precision%29))
  (bind _enemy (Variables|Default|GetEnemy))
  (bind _enemy_vec (Variables|/Game/SaveTheOcean/Enemy/BP_Parent_Enemy.BP_Parent_Enemy_C|GetEnemy_vec _enemy))
  ;[1 1 1] Enemy Vector
  (Utilities|FlowControl|Sequence
    (:then_0
      (Utilities|IsValid _enemy
        (:Is%20Valid
          (Variables|Default|SetTarget_Vector (Math|Vector|MakeVector (.x _enemy_vec) (- (.y _enemy_vec) 1.3e+02) (.z _enemy_vec))) ; 목표지점 설정
          (Variables|Default|SetPlayerVec (Transformation|GetActorLocation)))
        (:Is%20Not%20Valid
          (Development|PrintString "Failed!"))))
    (:then_1
      (Development|PrintString (Utilities|String|Append "HP : " (Utilities|String|ToString(Float) (Variables|Default|GetHealth%20Points%20HP))) true true "(R=0.074061,G=0.307292,B=0.138854,A=1.000000)" 0.0003))))

(fn ConstructionScript)

(fn VictoryCheck
  ;[1 0 0.07874] 적 체력 0 일 경우 VIctory 호출
  (if (<= (Variables|/Game/SaveTheOcean/Enemy/BP_Parent_Enemy.BP_Parent_Enemy_C|GetHealth (Variables|Default|GetEnemy)) 0.0)
    (CallFunction|VIctory)
    (return true)
    (else
      (Development|PrintString "The rest HP of Enemy :")
      (Development|PrintString (Utilities|String|ToString(Float) (Variables|/Game/SaveTheOcean/Enemy/BP_Parent_Enemy.BP_Parent_Enemy_C|GetHealth (Variables|Default|GetEnemy))))
      (return false))))