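; Player character for what appears to be turn-based combat against a single BP_Parent_Enemy, with stats copied from PlayerInfo on BeginPlay.
; Action events set a State enum, using timelines to dash toward the enemy, return and turn around, with delays pacing each action.
; Hit subtracts enemy power, Heal restores HP, Victory checks level-up, and Power Attack doubles offense before a later strike.
; Runaway is a stub and PowerUP's condition never passes.
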(event Custom|VIctory
  ;[1 1 1] #3 Victory (IncludeLvUpFunction)
  (Variables|Default|SetState "NewEnumerator4")
  (if (>= (+ (Variables|Default|GetExperience%20Point%20EXP) (Variables|/Game/SaveTheOcean/Enemy/BP_Parent_Enemy.BP_Parent_Enemy_C|GetEx (Variables|Default|GetEnemy))) (Variables|Default|GetLv_Up_EXP)) ; 레벨업 여부
    (Variables|Default|SetLv_Up_EXP (+ (Variables|Default|GetLv_Up_EXP) 1.0)) ; 레벨업에 따른 기준 경험치 상향조정
    (Variables|Default|SetPlayer%20Info%20Player%20Level (+ (Variables|Default|GetPlayer%20Info%20Player%20Level) 1))
    (Development|PrintString "Congratulations! You've gotten level up!"))
  (Utilities|FlowControl|Delay 2.0)
  (Variables|Default|SetState "NewEnumerator1"))

(event Custom|Attack
  (bind _startpoint (Variables|Default|GetStartPoint))
  (bind _target_vector (Variables|Default|GetTarget_Vector))
  ;[1 1 1] #1 Attack
  ;;[1 1 1] 캐릭터 전진
  (Variables|Default|SetState "NewEnumerator0")
  (bind _speed (Timeline|MoveForward PlayFromStart)
    (:Update
      (Transformation|SetActorLocation (+ (* (- (Variables|Default|GetTarget_Vector) _startpoint) _speed) _startpoint) false false))
    (:Finished
      ;;[1 1 1] 캐릭터 공격
      (Variables|Default|SetState "NewEnumerator2")
      (Utilities|FlowControl|Delay 2.6) ; 사운드넣기
      (if (Variables|Default|GetIs%20Enemy)
        (Utilities|FlowControl|Sequence
          (:then_0
            ;;[1 1 1] 원래 자리로 돌아가기
            (Variables|Default|SetState "NewEnumerator0")
            (bind _speed_2 (Timeline|Return PlayFromStart)
              (:Update
                (Transformation|SetActorLocation (+ (* (- (Variables|Default|GetStartPoint) _target_vector) _speed_2) _target_vector) false false))
              (:Finished
                (Variables|Default|SetState "NewEnumerator1")
                ;;[1 1 1] 캐릭터 회전
                (Variables|Default|SetReturn%20Value%20Z%20%28Yaw%29 (.yaw (Transformation|GetActorRotation)) :!label _label)
                (bind _rotation (Timeline|Turn_Physic PlayFromStart)
                  (:Update
                    (Transformation|SetActorRotation (Math|Rotator|MakeRotator 0.0 0.0 (Math|Float|Lerp (Variables|Default|GetReturn%20Value%20Z%20%28Yaw%29) (+ (Variables|Default|GetReturn%20Value%20Z%20%28Yaw%29) 1.8e+02) _rotation))))
                  (:Finished
                    ;;[1 1 1] If Enemy Down.
                    (if (<= (Variables|/Game/SaveTheOcean/Enemy/BP_Parent_Enemy.BP_Parent_Enemy_C|GetHealth (Variables|Default|GetEnemy)) 0.0)
                      (CallFunction|VIctory)
                      (else
                        (Development|PrintString "The rest HP of Enemy :")
                        (Development|PrintString (Utilities|String|ToString(Float) (Variables|/Game/SaveTheOcean/Enemy/BP_Parent_Enemy.BP_Parent_Enemy_C|GetHealth (Variables|Default|GetEnemy)))))))))))
          (:then_1
            (goto _label)))
        (else
          (Development|PrintString "It'sNotaEnemy"))))))

(event Custom|Heal
  ;[1 1 1] #5.1 Skill : Heal
  (if (> (Variables|Default|GetHealth%20Points%20HP) 0.0) ; IsPlayerAlive?
    (Variables|Default|SetState "NewEnumerator5")
    (Variables|Default|SetHealth%20Points%20HP (+ (Variables|Default|GetHealth%20Points%20HP) 1e+02))
    (Development|PrintString (Utilities|String|ToString(Float) (Variables|Default|GetHealth%20Points%20HP)))
    (Utilities|FlowControl|Delay 2.8)
    (Variables|Default|SetState "NewEnumerator1")
    (else
      (Development|PrintString (Utilities|String|ToString(Float) (Variables|Default|GetHealth%20Points%20HP)) true true "(R=0.000000,G=1.000000,B=0.184247,A=1.000000)"))))

(event Custom|Hit
  ;[1 1 1] #2 Hit
  (Variables|Default|SetState "NewEnumerator3")
  (Variables|Default|SetHealth%20Points%20HP (- (Variables|Default|GetHealth%20Points%20HP) (Variables|/Game/SaveTheOcean/Enemy/BP_Parent_Enemy.BP_Parent_Enemy_C|GetPower (Variables|Default|GetEnemy))))
  (Utilities|FlowControl|Delay 1.5)
  (if (> (Variables|Default|GetHealth%20Points%20HP) 0.0) ; IsPlayerAlive?
    (Variables|Default|SetState "NewEnumerator1")
    (else
      (Development|PrintString "You're dead" true true "(R=0.000000,G=1.000000,B=0.184247,A=1.000000)"))))

(event Custom|Stay
  ;[1 1 1] #4 Stay
  (Variables|Default|SetState "NewEnumerator1"))

(event Custom|Skill_PowerAttack
  (bind _target_vector (Variables|Default|GetTarget_Vector))
  (bind _startpoint (Variables|Default|GetStartPoint))
  ;[1 1 1] #5.2 Skill : Power Attack(with risk)
  (if (>= (Variables|Default|GetMana%20Points%20MP) 4e+01)
    (if (Variables|Default|GetIsPowerAttack)
      ;;[1 1 1] 캐릭터 전진
      (Variables|Default|SetState "NewEnumerator0")
      (bind _speed (Timeline|타임라인_0 PlayFromStart)
        (:Update
          (Transformation|SetActorLocation (+ (* (- (Variables|Default|GetTarget_Vector) _startpoint) _speed) _startpoint) false false))
        (:Finished
          ;;[1 1 1] 캐릭터 공격
          (Variables|Default|SetState "NewEnumerator6")
          (Utilities|FlowControl|Delay 2.6) ; 사운드넣기
          (if (not (Variables|Default|GetIs%20Enemy))
            (Development|PrintString "It'sNotaEnemy")
            (Utilities|FlowControl|Sequence
              (:then_0
                (Variables|Default|SetState "NewEnumerator0")
                (bind _speed_2 (Timeline|타임라인_2 PlayFromStart)
                  (:Update
                    (Transformation|SetActorLocation (+ (* (- (Variables|Default|GetStartPoint) _target_vector) _speed_2) _target_vector) false false))
                  (:Finished
                    (Variables|Default|SetState "NewEnumerator1")
                    ;;[1 1 1] 캐릭터 회전
                    (Variables|Default|SetReturn%20Value%20Z%20%28Yaw%29 (.yaw (Transformation|GetActorRotation)) :!label _label)
                    (bind _rotation (Timeline|타임라인_1 PlayFromStart)
                      (:Update
                        (Transformation|SetActorRotation (Math|Rotator|MakeRotator 0.0 0.0 (Math|Float|Lerp (Variables|Default|GetReturn%20Value%20Z%20%28Yaw%29) (+ (Variables|Default|GetReturn%20Value%20Z%20%28Yaw%29) 1.8e+02) _rotation))))
                      (:Finished
                        ;;[1 1 1] If Enemy Down.
                        (if (<= (Variables|/Game/SaveTheOcean/Enemy/BP_Parent_Enemy.BP_Parent_Enemy_C|GetHealth (Variables|Default|GetEnemy)) 0.0)
                          (CallFunction|VIctory)
                          (else
                            (Development|PrintString "The rest HP of Enemy :")
                            (Development|PrintString (Utilities|String|ToString(Float) (Variables|/Game/SaveTheOcean/Enemy/BP_Parent_Enemy.BP_Parent_Enemy_C|GetHealth (Variables|Default|GetEnemy)))))))))))
              (:then_1
                (goto _label))
              (:then_2
                (Variables|Default|SetIsPowerAttack false) ; 강타상태였을 경우 파워업 해제
                (Variables|Default|SetOffense%20Power%20AD 1e+01) ; 공격력 원상회복
              )))))
      (else
        (Variables|Default|SetIsPowerAttack true)
        (Variables|Default|SetOffense%20Power%20AD (* (Variables|Default|GetOffense%20Power%20AD) 2.0)) ; 공격사용시까지 공격력 2배 증가
        (Development|PrintString "The power attack is ready for use")))
    (else
      (Development|PrintString "You've not enogh MP."))))

(event Custom|PowerUP
  ;[1 1 1] #5.4 Skill : Power UP
  (if (>= 0.0 4e+01)
    (Variables|Default|SetIsPowerAttack true)
    (Variables|Default|SetOffense%20Power%20AD (* (Variables|Default|GetOffense%20Power%20AD) 2.0)) ; 공격사용시까지 공격력 2배 증가
    (Development|PrintString "The power attack is ready for use")))

(event Custom|Runaway
  ;[1 1 1] #6 RunAway
  (if (> (Variables|Default|GetHealth%20Points%20HP) 0.0)
    _))

(event EventBeginPlay
  (bind _playerinfo (Variables|Default|GetPlayerInfo))
  (bind (_playerlevel _healthpoints_hp _manapoints_mp _experiencepoint_exp _offensepower_ad) (Utilities|Struct|BreakBP_PlayerInfo _playerinfo))
  ;[1 1 1] #0 Set the Player Info
  (Variables|Default|SetPlayer%20Info%20Player%20Level _playerlevel)
  (Variables|Default|SetHealth%20Points%20HP _healthpoints_hp)
  (Variables|Default|SetMana%20Points%20MP _manapoints_mp)
  (Variables|Default|SetExperience%20Point%20EXP _experiencepoint_exp)
  (Variables|Default|SetOffense%20Power%20AD _offensepower_ad)
  (bind _returnvalue (Actor|GetActorOfClass "/Game/SaveTheOcean/Enemy/BP_Parent_Enemy.BP_Parent_Enemy_C"))
  (Variables|Default|SetEnemy _returnvalue)
  (Variables|Default|SetStartPoint (Transformation|GetActorLocation)))

(event EventTick
  (params (DeltaSeconds :type Float%20%28single-precision%29))
  (bind _enemy (Variables|Default|GetEnemy))
  (bind _enemy_vec (Variables|/Game/SaveTheOcean/Enemy/BP_Parent_Enemy.BP_Parent_Enemy_C|GetEnemy_vec _enemy))
  ;[1 1 1] Enemy Vector
  (Utilities|IsValid _enemy
    (:Is%20Valid
      (Variables|Default|SetTarget_Vector (Math|Vector|MakeVector (.x _enemy_vec) (- (.y _enemy_vec) 1.3e+02) (.z _enemy_vec))) ; 목표지점 설정
      (Variables|Default|SetPlayerVec (Transformation|GetActorLocation)))))

(fn ConstructionScript)