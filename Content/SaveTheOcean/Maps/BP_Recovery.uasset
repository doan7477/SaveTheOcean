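; BP_Recovery is a healing zone that restores a BP_MovePlayer's HP and MP while they stand inside it.
; Overlap begin stores the player and shows their HealParticle; overlap end hides it, clears the reference and calls SaveFieldInfo on the game instance.
; While the reference is valid, Tick adds a fixed, frame-rate-dependent amount to MovePlayerInfo, clamping HP to a constant cap and MP to a cap selected by player level.
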(event EventBeginPlay)

(event Collision|EventActorBeginOverlap
  (params (OtherActor :type Actor%20Object%20Reference))
  ;[1 1 1] 컬리전박스 들어갈때 MovePlayerRef변수에 BP_MovePlayer값을 넣어준 후 힐 이펙트를 켜줌
  (bind _asbp_move_player (Utilities|Casting|CastToBP_MovePlayer OtherActor))
  (bind _output_get (Variables|Default|SetMovePlayer_Ref _asbp_move_player))
  (Rendering|SetVisibility (Variables|/Game/SaveTheOcean/Player/Move/BP_MovePlayer.BP_MovePlayer_C|GetHealParticle _output_get) true false))

(event EventTick
  (params (DeltaSeconds :type Float%20%28single-precision%29))
  (bind _moveplayer_ref (Variables|Default|GetMovePlayer_Ref))
  ;[1 1 1] MovePlayerRef변수에 값이 들어있는지 아닌지(유효한지) 검사
  (Utilities|IsValid (Variables|Default|GetMovePlayer_Ref)
    (:Is%20Valid
      (Variables|/Game/SaveTheOcean/Player/Move/BP_MovePlayer.BP_MovePlayer_C|SetMovePlayerInfo _moveplayer_ref (Utilities|Struct|MakeBP_PlayerInfo (.playerlevel (Variables|/Game/SaveTheOcean/Player/Move/BP_MovePlayer.BP_MovePlayer_C|GetMovePlayerInfo _moveplayer_ref)) (Math|Float|Clamp(Float) (+ (.healthpoints_hp (Variables|/Game/SaveTheOcean/Player/Move/BP_MovePlayer.BP_MovePlayer_C|GetMovePlayerInfo _moveplayer_ref)) 0.5) 0.0 1e+02) (Math|Float|Clamp(Float) (+ (.manapoints_mp (Variables|/Game/SaveTheOcean/Player/Move/BP_MovePlayer.BP_MovePlayer_C|GetMovePlayerInfo _moveplayer_ref)) 0.5) 0.0 (Utilities|Select :Index (.playerlevel (Variables|/Game/SaveTheOcean/Player/Move/BP_MovePlayer.BP_MovePlayer_C|GetMovePlayerInfo _moveplayer_ref)) :Option%200 45.0 :Option%201 45.0 :Option%202 7e+01 :Option%203 1e+02)) (.experiencepoint_exp (Variables|/Game/SaveTheOcean/Player/Move/BP_MovePlayer.BP_MovePlayer_C|GetMovePlayerInfo _moveplayer_ref)) (.offensepower_ad (Variables|/Game/SaveTheOcean/Player/Move/BP_MovePlayer.BP_MovePlayer_C|GetMovePlayerInfo _moveplayer_ref)))))))

(event Collision|EventActorEndOverlap
  (params (OtherActor :type Actor%20Object%20Reference))
  ;[1 1 1] 컬리전박스 나올때 힐 이펙트를 꺼주고 MovePlayerRef변수에 값이 들어있던 것을 빈 값으로 되돌림
  (if (== OtherActor (Variables|Default|GetMovePlayer_Ref))
    (Rendering|SetVisibility (Variables|/Game/SaveTheOcean/Player/Move/BP_MovePlayer.BP_MovePlayer_C|GetHealParticle (Variables|Default|GetMovePlayer_Ref)) false false)
    (Variables|Default|SetMovePlayer_Ref 0)
    ;[1 1 1] Save 관련
    (bind _assave_the_ocean_game_instance (Utilities|Casting|CastToSaveTheOceanGameInstance (Game|GetGameInstance)))
    (Default|SaveFieldInfo _assave_the_ocean_game_instance)))

(fn ConstructionScript)