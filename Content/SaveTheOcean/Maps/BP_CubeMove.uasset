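; BP_CubeMove is an actor that the player moves horizontally with axis input.
; On BeginPlay it enables input from player controller 0.
; The MoveLeftRight and MoveForwardBackward axes each add a fixed step along world Y and X, scaled by the axis value, to the actor location.
; Movement uses SetActorLocation without sweep or delta-time scaling, so it ignores collision and depends on frame rate.
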(event EventBeginPlay
  ;[1 1 1] 입력 활성화
  (Input|EnableInput (Game|GetPlayerController 0)))

(event Collision|EventActorBeginOverlap
  (params (OtherActor :type Actor%20Object%20Reference)))

(event EventTick
  (params (DeltaSeconds :type Float%20%28single-precision%29)))

(event Input|AxisEvents|InputAxisMoveLeftRight
  (params (AxisValue :type Float%20%28single-precision%29))
  ;[1 1 1] 좌우이동
  (Transformation|SetActorLocation (+ (* "0,5.000000, 0" AxisValue) (Transformation|GetActorLocation)) false false))

(event Input|AxisEvents|InputAxisMoveForwardBackward
  (params (AxisValue :type Float%20%28single-precision%29))
  ;[1 1 1] 앞뒤 이동
  (Transformation|SetActorLocation (+ (* "5.000000,0.000000, 0" AxisValue) (Transformation|GetActorLocation)) false false))

(fn ConstructionScript)