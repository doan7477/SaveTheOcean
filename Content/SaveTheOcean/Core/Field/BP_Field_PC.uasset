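; BP_Field_PC is the player controller for the field in SaveTheOcean, restoring the player's saved state on start.
; BeginPlay hides the cursor, sets game-only input, and loads save data through SaveTheOceanGameInstance.
; It then copies the saved player info to the BP_MovePlayer character and moves it to the saved field location.
; Key 1 overwrites one player stat with a fixed value, apparently a debug shortcut.
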(event EventBeginPlay
  ;[1 1 1] UI
  (Variables|Default|SetbShowMouseCursor false)
  (Input|SetInputModeGameOnly self)
  ;[1 1 1] Save Data 가져오기
  (bind _assave_the_ocean_game_instance (Utilities|Casting|CastToSaveTheOceanGameInstance (Game|GetGameInstance)))
  (Default|LoadSaveData _assave_the_ocean_game_instance)
  ;[1 1 1] Move Player에 값 넣어주기
  (bind _asbp_move_player (Utilities|Casting|CastToBP_MovePlayer (Game|GetPlayerCharacter 0)))
  (Variables|/Game/SaveTheOcean/Player/Move/BP_MovePlayer.BP_MovePlayer_C|SetMovePlayerInfo _asbp_move_player (Variables|/Game/SaveTheOcean/Core/SaveGameBP.SaveGameBP_C|GetPlayerInfo (Variables|/Game/SaveTheOcean/Core/SaveTheOceanGameInstance.SaveTheOceanGameInstance_C|GetSaveData _assave_the_ocean_game_instance)))
  (Transformation|SetActorLocation _asbp_move_player (Variables|/Game/SaveTheOcean/Core/SaveGameBP.SaveGameBP_C|GetFieldPlayerLocation (Variables|/Game/SaveTheOcean/Core/SaveTheOceanGameInstance.SaveTheOceanGameInstance_C|GetSaveData _assave_the_ocean_game_instance)) false false))

(event EventTick
  (params (DeltaSeconds :type Float%20%28single-precision%29)))

(event Input|KeyboardEvents|1
  (params (Key :type Key%20Structure :default "None"))
  (:Pressed
    (bind _asbp_move_player (Utilities|Casting|CastToBP_MovePlayer (Game|GetPlayerCharacter 0)))
    (Variables|/Game/SaveTheOcean/Player/Move/BP_MovePlayer.BP_MovePlayer_C|SetMovePlayerInfo _asbp_move_player (Utilities|Struct|MakeBP_PlayerInfo (.playerlevel (Variables|/Game/SaveTheOcean/Player/Move/BP_MovePlayer.BP_MovePlayer_C|GetMovePlayerInfo _asbp_move_player)) 5e+01 (.manapoints_mp (Variables|/Game/SaveTheOcean/Player/Move/BP_MovePlayer.BP_MovePlayer_C|GetMovePlayerInfo _asbp_move_player)) (.experiencepoint_exp (Variables|/Game/SaveTheOcean/Player/Move/BP_MovePlayer.BP_MovePlayer_C|GetMovePlayerInfo _asbp_move_player)) (.offensepower_ad (Variables|/Game/SaveTheOcean/Player/Move/BP_MovePlayer.BP_MovePlayer_C|GetMovePlayerInfo _asbp_move_player))))))

(fn ConstructionScript)