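; Base enemy Blueprint for what appears to be turn-based combat, with Attack, Hit, Skill and Heal events.
; BeginPlay copies EnemyStatus stats and caches BP_Player; Tick tracks a point offset in front of the player.
; Attack runs timelines to lunge there and back, subtracting Power × Level from player health immediately.
; Skill and Heal spend mana; a State enum, often reset by delays, marks actions and death.
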(event Custom|Heal
  ;[0.4973 1 0.531] Heal
  (if (>= (Variables|Default|GetMana%20Point) 50) ; 마나가 50 이상일 때에만 Heal 사용
    (Variables|Default|SetState "NewEnumerator5")
    (bind _output_get (Variables|Default|SetHealth (+ (Variables|Default|GetHealth) 30))) ; HP 회복
    (bind _output_get_2 (Variables|Default|SetMana%20Point (- (Variables|Default|GetMana%20Point) 50))) ; MP 차감
    (Development|PrintString "EnemyHP :" true true "(R=0.000000,G=0.660000,B=1.000000,A=1.000000)" 3.0)
    (Development|PrintString (Utilities|String|ToString(Integer) _output_get) true true "(R=0.000000,G=0.660000,B=1.000000,A=1.000000)" 3.0)
    (Development|PrintString "EnemyMP :" true true "(R=0.011612,G=0.000000,B=1.000000,A=1.000000)" 3.0)
    (Development|PrintString (Utilities|String|ToString(Integer) _output_get_2) true true "(R=0.011612,G=0.000000,B=1.000000,A=1.000000)" 3.0)
    (Utilities|FlowControl|Delay 3.0)
    (Variables|Default|SetState "NewEnumerator0")
    (else
      (Development|PrintString "MP is not enough to use skill" true true "(R=0.011612,G=0.000000,B=1.000000,A=1.000000)"))))

(event Custom|Hit
  ;[1 0.604 0.7793] Hit
  (Variables|Default|SetHealth (- (Variables|Default|GetHealth) 30))
  (Variables|Default|SetState "NewEnumerator2")
  (Utilities|FlowControl|Delay 0.5)
  ;;[1 0.1107 0.1904] Dead
  (if (<= (Variables|Default|GetHealth) 0) ; 체력이 0이하이면 Dead 모션 출력
    (Variables|Default|SetState "NewEnumerator3")
    (Development|PrintString (Variables|Default|GetName) true true "(R=1.000000,G=0.000000,B=0.047235,A=1.000000)")
    (Development|PrintString " Dead" true true "(R=1.000000,G=0.000000,B=0.047235,A=1.000000)")
    (else
      (Variables|Default|SetState "NewEnumerator0")
      (if (<= (Variables|Default|GetHealth) 0)
        (bind _output_get (Variables|Default|SetHealth (Variables|Default|GetHealth))))
      (Development|PrintString "EnemyHP :" true true "(R=0.000000,G=0.660000,B=1.000000,A=1.000000)" 3.0)
      (Development|PrintString (Utilities|String|ToString(Integer) _output_get) true true "(R=0.000000,G=0.660000,B=1.000000,A=1.000000)" 3.0))))

(event Custom|Skill
  (bind _player (Variables|Default|GetPlayer))
  ;[1 1 1] Skill - Dot Damage
  (if (>= (Variables|Default|GetMana%20Point) 40) ; 마나가 40 이상일 때에만 skill 사용
    (Variables|Default|SetMana%20Point (- (Variables|Default|GetMana%20Point) 40)) ; MP 차감
    ;;[0.2195 0.3712 1] Player
    (bind _output_get (Variables|/Game/SaveTheOcean/Enemy/BP_Player.BP_Player_C|SetHealth _player (- (Variables|/Game/SaveTheOcean/Enemy/BP_Player.BP_Player_C|GetHealth _player) (/ (Variables|Default|GetPower) 5))))
    (Development|PrintString "PlayerHP :" true true "(R=0.000000,G=0.660000,B=1.000000,A=1.000000)" 3.0)
    (Development|PrintString (Utilities|String|ToString(Integer) _output_get) true true "(R=0.000000,G=0.660000,B=1.000000,A=1.000000)" 3.0)
    (else
      (Development|PrintString "MP is not enough to use skill" true true "(R=0.011612,G=0.000000,B=1.000000,A=1.000000)"))))

(event Custom|Attack
  (bind _player (Variables|Default|GetPlayer))
  ;[1 1 1] Attack
  (Variables|Default|Setstartpoint_Vector (Transformation|GetActorLocation))
  (Utilities|FlowControl|Sequence
    (:then_0
      (bind _speed (Timeline|타임라인_0 PlayFromStart)
        (:Update
          (Transformation|SetActorLocation (+ (* (- (Variables|Default|GetTarget_Vector) (Variables|Default|Getstartpoint_Vector)) _speed) (Variables|Default|Getstartpoint_Vector)) false false)
          ;[1 1 1] Animation
          (Variables|Default|SetState "NewEnumerator1")
          (Utilities|FlowControl|Delay 0.9)
          (Variables|Default|SetState "NewEnumerator0"))))
    (:then_1
      ;[1 1 1] Damage Check
      ;;[0.2195 0.3712 1] Player
      (bind _output_get (Variables|/Game/SaveTheOcean/Enemy/BP_Player.BP_Player_C|SetHealth _player (- (Variables|/Game/SaveTheOcean/Enemy/BP_Player.BP_Player_C|GetHealth _player) (* (Variables|Default|GetPower) (Variables|Default|GetLevel)))))
      (Development|PrintString "PlayerHP :" true true "(R=0.000000,G=0.660000,B=1.000000,A=1.000000)" 3.0)
      (Development|PrintString (Utilities|String|ToString(Integer) _output_get) true true "(R=0.000000,G=0.660000,B=1.000000,A=1.000000)" 3.0))
    (:then_2
      (Utilities|FlowControl|Delay 2.0)
      (bind _speed_2 (Timeline|타임라인_1 PlayFromStart)
        (:Update
          (Transformation|SetActorLocation (+ (* (- (Variables|Default|Getstartpoint_Vector) (Variables|Default|GetTarget_Vector)) _speed_2) (Variables|Default|GetTarget_Vector)) false false)
          (Variables|Default|SetState "NewEnumerator4")
          (Utilities|FlowControl|Delay 1.0)
          (Variables|Default|SetState "NewEnumerator0"))))))

(event EventBeginPlay
  (bind _enemystatus (Variables|Default|GetEnemyStatus))
  (bind (_name _level _healthpoint _manapoint _ex _power) (Utilities|Struct|BreakEnemyInfo _enemystatus))
  ;[1 1 1] Setting
  (Variables|Default|SetName _name) ; 기본 status 변수로 저장
  (Variables|Default|SetLevel _level)
  (Variables|Default|SetEx _ex)
  (Variables|Default|SetHealth _healthpoint)
  (Variables|Default|SetMana%20Point _manapoint)
  (Variables|Default|SetPower _power)
  (bind _returnvalue (Actor|GetActorOfClass "/Game/SaveTheOcean/Enemy/BP_Player.BP_Player_C")) ; 플레이어 캐릭터 위치값 가져오기
  (Variables|Default|SetPlayer _returnvalue) ; 변수 승격
)

(event Collision|EventActorBeginOverlap
  (params (OtherActor :type Actor%20Object%20Reference)))

(event EventTick
  (params (DeltaSeconds :type Float%20%28single-precision%29))
  (bind _player (Variables|Default|GetPlayer))
  (bind _player_vector (Variables|/Game/SaveTheOcean/Enemy/BP_Player.BP_Player_C|GetPlayer_Vector _player))
  ;[1 1 1] Target Check
  ;;[0.2195 0.3712 1] Player
  (Utilities|IsValid _player
    (:Is%20Valid
      (Variables|Default|SetTarget_Vector (Math|Vector|MakeVector (.x _player_vector) (- (.y _player_vector) 1.3e+02) (.z _player_vector))) ; 목표지점 설정
    )
    (:Is%20Not%20Valid
      (Development|PrintString "Player BP is not Valid" true true "(R=0.000000,G=0.660000,B=1.000000,A=1.000000)" 1e+02))))

(fn ConstructionScript)