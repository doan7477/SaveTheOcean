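; BP_child_Boss is a child enemy Blueprint for the boss, overriding the Skill event with a charge move that raises Power instead of attacking.
; Skill plays the boss skill Level Sequence, spends mana, adds to Power and shows SkillEffect.
; It also switches State, then changes it again after a short delay.
; BeginPlay, Tick and construction defer to the parent class.
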(event EventBeginPlay
  (|CallParentFunction))

(event Collision|EventActorBeginOverlap
  (params (OtherActor :type Actor%20Object%20Reference))
  (|CallParentFunction OtherActor) ; 지금 이 노드는 비활성 상태입니다. \n핀을 끌어서 다른 노드를 연결하면 활성화됩니다.
)

(event EventTick
  (params (DeltaSeconds :type Float%20%28single-precision%29))
  (|CallParentFunction DeltaSeconds))

(event EventSkill
  ;[1 1 1] Skill_Charge
  (Utilities|FlowControl|Sequence
    (:then_0
      ;[1 0.9803 0] 스킬 시퀀스 재생
      (bind _returnvalue (Sequencer|Player|CreateLevelSequencePlayer "/Game/SaveTheOcean/Player/Battle/Battle_Sequence/Enemy/Battle_Sequence_Enemy_Skill_Boss.Battle_Sequence_Enemy_Skill_Boss"))
      (Sequencer|Player|Play _returnvalue :!class /Script/MovieScene.MovieSceneSequencePlayer)
      (Variables|Default|SetMana%20Point (- (Variables|Default|GetMana%20Point) 4e+01)) ; MP 차감
      (Variables|Default|SetPower (+ (Variables|Default|GetPower) 2e+01)) ; 최종 데미지 더하기.  공격은 안함
      (Rendering|SetVisibility (Variables|Default|GetSkillEffect) true false))
    (:then_1
      (Variables|Default|SetState "NewEnumerator6")
      (Utilities|FlowControl|Delay 2.0)
      (Variables|Default|SetState "NewEnumerator0"))))

(fn ConstructionScript
  (|CallParentFunction))