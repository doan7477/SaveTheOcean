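; BP_Ch_TrashMan is an enemy character that makes one attack on BP_Player_test at BeginPlay.
; Tick keeps a target point offset in front of the player, and two timelines move it there and, after a delay, back to its start.
; Attack subtracts its Power from player health immediately, without waiting for the lunge.
; Hit removes fixed health, and both events switch an enum State for animation, including death.
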(event Custom|Hit
  ;[1 1 1] Hit
  (Utilities|FlowControl|Sequence
    (:then_0
      (Variables|Default|SetHealth (- (Variables|Default|GetHealth) 30))
      (Variables|Default|SetState "NewEnumerator2")
      (Utilities|FlowControl|Delay 0.5)
      (Variables|Default|SetState "NewEnumerator0")
      (if (<= (Variables|Default|GetHealth) 0)
        (Variables|Default|SetHealth 0))
      (Development|PrintString "EnemyHP :" true true "(R=0.000000,G=0.660000,B=1.000000,A=1.000000)" 3.0)
      (Development|PrintString (Utilities|String|ToString(Integer) (Variables|Default|GetHealth)) true true "(R=0.000000,G=0.660000,B=1.000000,A=1.000000)" 3.0))
    (:then_1
      ;[1 1 1] Dead
      (if (<= (Variables|Default|GetHealth) 0)
        (Variables|Default|SetState "NewEnumerator3")
        (Development|PrintString "TrashMan Dead")))))

(event Custom|Attack
  (bind _player_bp (Variables|Default|GetPlayer_BP))
  ;[1 1 1] Attack
  (Variables|Default|Setstartpoint_Vector (Transformation|GetActorLocation))
  (Utilities|FlowControl|Sequence
    (:then_0
      (bind _speed (Timeline|타임라인_0 Play)
        (:Update
          (Transformation|SetActorLocation (+ (* (- (Variables|Default|GetTarget_Vector) (Variables|Default|Getstartpoint_Vector)) _speed) (Variables|Default|Getstartpoint_Vector)) false false)
          ;[1 1 1] Animation
          (Variables|Default|SetState "NewEnumerator1")
          (Utilities|FlowControl|Delay 0.9)
          (Variables|Default|SetState "NewEnumerator0"))))
    (:then_1
      (Utilities|FlowControl|Delay 2.0)
      (bind _speed_2 (Timeline|타임라인_1 PlayFromStart)
        (:Update
          (Transformation|SetActorLocation (+ (* (- (Variables|Default|Getstartpoint_Vector) (Variables|Default|GetTarget_Vector)) _speed_2) (Variables|Default|GetTarget_Vector)) false false)
          (Variables|Default|SetState "NewEnumerator4")
          (Utilities|FlowControl|Delay 1.0)
          (Variables|Default|SetState "NewEnumerator0"))))
    (:then_2
      ;[1 1 1] Damage Check
      (bind _output_get (Variables|/Game/SaveTheOcean/Enemy/BP_Player_test.BP_Player_test_C|SetPlayer_Health _player_bp (- (Variables|/Game/SaveTheOcean/Enemy/BP_Player_test.BP_Player_test_C|GetPlayer_Health _player_bp) (.Power (Utilities|Struct|BreakEnemyInfo (Variables|Default|GetEnemyStatus))))))
      (Development|PrintString "PlayerHP :" true true "(R=0.000000,G=0.660000,B=1.000000,A=1.000000)" 3.0)
      (Development|PrintString (Utilities|String|ToString(Integer) _output_get) true true "(R=0.000000,G=0.660000,B=1.000000,A=1.000000)" 3.0))))

(event EventBeginPlay
  (Variables|Default|SetHealth (.HealthPoint (Utilities|Struct|BreakEnemyInfo (Variables|Default|GetEnemyStatus))))
  (bind _returnvalue (Actor|GetActorOfClass "/Game/SaveTheOcean/Enemy/BP_Player_test.BP_Player_test_C")) ; 플레이어 캐릭터 위치값 가져오기
  (Variables|Default|SetPlayer_BP _returnvalue)
  (CallFunction|Attack))

(event Collision|EventActorBeginOverlap
  (params (OtherActor :type Actor%20Object%20Reference)))

(event EventTick
  (params (DeltaSeconds :type Float%20%28single-precision%29))
  (bind _player_bp (Variables|Default|GetPlayer_BP))
  (bind _player_vector (Variables|/Game/SaveTheOcean/Enemy/BP_Player_test.BP_Player_test_C|GetPlayer_Vector _player_bp))
  ;[1 1 1] Target Check
  (Utilities|IsValid _player_bp
    (:Is%20Valid
      (Variables|Default|SetTarget_Vector (Math|Vector|MakeVector (.x _player_vector) (- (.y _player_vector) 1.3e+02) (.z _player_vector))) ; 목표지점 설정
    )
    (:Is%20Not%20Valid
      (Development|PrintString "Player BP is not Valid" true true "(R=0.000000,G=0.660000,B=1.000000,A=1.000000)" 1e+02))))

(fn ConstructionScript)