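; BP_Enemy1 is a TrashMan enemy that makes one scripted lunge at the player on BeginPlay and returns to its start.
; Tick keeps a target point offset in Y from BP_Player_test.
; Attack saves the origin, interpolates out and, after a delay, back via timelines, setting TrashMan_AnimBP's Speed along the way.
; Player health is reduced as soon as Attack starts, with no hit or overlap check.
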(event Custom|Attack
  ;[1 1 1] Attack
  (Variables|Default|Setstartpoint_Vector (Transformation|GetActorLocation))
  (Utilities|FlowControl|Sequence
    (:then_0
      (bind _speed (Timeline|타임라인_0 Play)
        (:Update
          (Transformation|SetActorLocation (+ (* (- (Variables|Default|GetTarget_Vector) (Variables|Default|Getstartpoint_Vector)) _speed) (Variables|Default|Getstartpoint_Vector)) false false)
          ;[1 1 1] Animation
          (bind _astrash_man_anim_bp (Utilities|Casting|CastToTrashMan_AnimBP (Components|SkeletalMesh|GetAnimInstance (Variables|Default|GetTrashMan))))
          (Variables|/Game/SaveTheOcean/Enemy/Model/TrashMan/TrashMan_AnimBP.TrashMan_AnimBP_C|SetSpeed _astrash_man_anim_bp 5e+01)
          (Utilities|FlowControl|Delay 0.9)
          (bind _새_트랙_0 (Timeline|타임라인_2 ReverseFromEnd)))))
    (:then_1
      (Utilities|FlowControl|Delay 2.0)
      (bind _speed_2 (Timeline|타임라인_1 PlayFromStart)
        (:Update
          (Transformation|SetActorLocation (+ (* (- (Variables|Default|Getstartpoint_Vector) (Variables|Default|GetTarget_Vector)) _speed_2) (Variables|Default|GetTarget_Vector)) false false)
          (bind _astrash_man_anim_bp_2 (Utilities|Casting|CastToTrashMan_AnimBP (Components|SkeletalMesh|GetAnimInstance (Variables|Default|GetTrashMan))))
          (Variables|/Game/SaveTheOcean/Enemy/Model/TrashMan/TrashMan_AnimBP.TrashMan_AnimBP_C|SetSpeed _astrash_man_anim_bp_2 1e+02)
          (Utilities|FlowControl|Delay 1.0)
          (bind _astrash_man_anim_bp_3 (Utilities|Casting|CastToTrashMan_AnimBP (Components|SkeletalMesh|GetAnimInstance (Variables|Default|GetTrashMan))))
          (Variables|/Game/SaveTheOcean/Enemy/Model/TrashMan/TrashMan_AnimBP.TrashMan_AnimBP_C|SetSpeed _astrash_man_anim_bp_3 0.0))))
    (:then_2
      ;[1 1 1] Damage Check
      (bind _returnvalue (Actor|GetActorOfClass "/Game/SaveTheOcean/Enemy/BP_Player_test.BP_Player_test_C")) ; 플레이어 BP 에서 체력값 가져오기
      (bind _asbp_player_test (Utilities|Casting|CastToBP_Player_test _returnvalue))
      (Variables|/Game/SaveTheOcean/Enemy/BP_Player_test.BP_Player_test_C|SetPlayer_Health _asbp_player_test (- (Variables|/Game/SaveTheOcean/Enemy/BP_Player_test.BP_Player_test_C|GetPlayer_Health _asbp_player_test) 30)))))

(event EventBeginPlay
  (CallFunction|Attack))

(event Collision|EventActorBeginOverlap
  (params (OtherActor :type Actor%20Object%20Reference)))

(event EventTick
  (params (DeltaSeconds :type Float%20%28single-precision%29))
  ;[1 1 1] Target Check
  (bind _returnvalue (Actor|GetActorOfClass "/Game/SaveTheOcean/Enemy/BP_Player_test.BP_Player_test_C")) ; 플레이어 캐릭터 위치값 가져오기
  (bind _asbp_player_test (Utilities|Casting|CastToBP_Player_test _returnvalue))
  (Variables|Default|SetTarget_Vector (Math|Vector|MakeVector (.x (Variables|/Game/SaveTheOcean/Enemy/BP_Player_test.BP_Player_test_C|GetPlayer_Vector _asbp_player_test)) (- (.y (Variables|/Game/SaveTheOcean/Enemy/BP_Player_test.BP_Player_test_C|GetPlayer_Vector _asbp_player_test)) 1.3e+02) (.z (Variables|/Game/SaveTheOcean/Enemy/BP_Player_test.BP_Player_test_C|GetPlayer_Vector _asbp_player_test)))) ; 목표지점 설정
)

(fn ConstructionScript)