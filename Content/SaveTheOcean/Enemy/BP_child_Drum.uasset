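; Drum enemy child Blueprint that defers to its parent for base behavior and adds a strong-attack Skill.
; Skill spends mana, adds level-scaled damage to Power and saves the start location.
; One timeline lerps the actor to TargetVector and calls the player's Hit after a delay; a second, delayed timeline returns it.
; State changes accompany each phase, while Tick offsets TargetVector's Y as long as Useskill is set.
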(event EventBeginPlay
  (|CallParentFunction))

(event Collision|EventActorBeginOverlap
  (params (OtherActor :type Actor%20Object%20Reference))
  (|CallParentFunction OtherActor) ; 지금 이 노드는 비활성 상태입니다. \n핀을 끌어서 다른 노드를 연결하면 활성화됩니다.
)

(event EventTick
  (params (DeltaSeconds :type Float%20%28single-precision%29))
  (|CallParentFunction DeltaSeconds)
  (if (Variables|Default|Getuseskill)
    (Variables|Default|SetTarget_Vector (Math|Vector|MakeVector (.x (Variables|Default|GetTarget_Vector)) (- (.y (Variables|Default|GetTarget_Vector)) -5e+01) (.z (Variables|Default|GetTarget_Vector))))))

(event EventSkill
  ;[1 1 1] Skill - strong attack
  (Utilities|FlowControl|Sequence
    (:then_0
      (Variables|Default|SetMana%20Point (- (Variables|Default|GetMana%20Point) 4e+01)) ; MP 차감
      (Variables|Default|SetPower (+ (Variables|Default|GetPower) (Math|Conversions|ToFloat(Integer) (* (Variables|Default|GetLevel) 10)))) ; 레벨 당 데미지 추가 후 바로 공격
      (Variables|Default|Setuseskill true)
      ;[1 1 1] Move
      (Variables|Default|Setstartpoint_Vector (Transformation|GetActorLocation))
      (Utilities|FlowControl|Sequence
        (:then_0
          (bind _speed (Timeline|타임라인_2 PlayFromStart)
            (:Update
              (Transformation|SetActorLocation (+ (* (- (Variables|Default|GetTarget_Vector) (Variables|Default|Getstartpoint_Vector)) _speed) (Variables|Default|Getstartpoint_Vector)) false false)
              (Variables|Default|SetState "NewEnumerator6")
              (Utilities|FlowControl|Sequence
                (:then_0
                  (Utilities|FlowControl|Delay 1.4)
                  (Default|Hit (Variables|Default|GetMainPlayer) 0.0))
                (:then_1
                  (Utilities|FlowControl|Delay 2.0)
                  (Variables|Default|SetState "NewEnumerator0"))))))
        (:then_1
          (Utilities|FlowControl|Delay 2.0)
          (bind _speed_2 (Timeline|타임라인_3 PlayFromStart)
            (:Update
              (Transformation|SetActorLocation (+ (* (- (Variables|Default|Getstartpoint_Vector) (Variables|Default|GetTarget_Vector)) _speed_2) (Variables|Default|GetTarget_Vector)) false false)
              (Variables|Default|SetState "NewEnumerator4")
              (Utilities|FlowControl|Delay 1.0)
              (Variables|Default|SetState "NewEnumerator0")
              (Variables|Default|Setuseskill false))))))))

(fn ConstructionScript
  (|CallParentFunction))