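; BP_Enemy is an enemy that makes one lunge-and-return attack on BP_Player_test when it spawns.
; Tick keeps the target at a fixed Y offset from the player's stored position.
; Attack uses two timelines to move the enemy toward that target, then back to its start after a delay.
; Its Sequence also subtracts player health immediately, without waiting for the lunge or checking overlap.
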(event Custom|Attack
  ;[1 1 1] Attack
  (Variables|Default|Setstartpoint_Vector (Transformation|GetActorLocation))
  (Utilities|FlowControl|Sequence
    (:then_0
      (bind _speed (Timeline|타임라인_0 Play)
        (:Update
          (Transformation|SetActorLocation (+ (* (- (Variables|Default|GetTarget_Vector) (Variables|Default|Getstartpoint_Vector)) _speed) (Variables|Default|Getstartpoint_Vector)) false false))))
    (:then_1
      (Utilities|FlowControl|Delay 2.0)
      (bind _speed_2 (Timeline|타임라인_1 PlayFromStart)
        (:Update
          (Transformation|SetActorLocation (+ (* (- (Variables|Default|Getstartpoint_Vector) (Variables|Default|GetTarget_Vector)) _speed_2) (Variables|Default|GetTarget_Vector)) false false))))
    (:then_2
      (bind _returnvalue (Actor|GetActorOfClass "/Game/SaveTheOcean/Enemy/BP_Player_test.BP_Player_test_C"))
      (bind _asbp_player_test (Utilities|Casting|CastToBP_Player_test _returnvalue))
      (Variables|/Game/SaveTheOcean/Enemy/BP_Player_test.BP_Player_test_C|SetPlayer_Health _asbp_player_test (- (Variables|/Game/SaveTheOcean/Enemy/BP_Player_test.BP_Player_test_C|GetPlayer_Health _asbp_player_test) 30)))))

(event EventBeginPlay
  (CallFunction|Attack))

(event Collision|EventActorBeginOverlap
  (params (OtherActor :type Actor%20Object%20Reference)))

(event EventTick
  (params (DeltaSeconds :type Float%20%28single-precision%29))
  (bind _returnvalue (Actor|GetActorOfClass "/Game/SaveTheOcean/Enemy/BP_Player_test.BP_Player_test_C"))
  (bind _asbp_player_test (Utilities|Casting|CastToBP_Player_test _returnvalue))
  (Variables|Default|SetTarget_Vector (Math|Vector|MakeVector (.x (Variables|/Game/SaveTheOcean/Enemy/BP_Player_test.BP_Player_test_C|GetPlayer_Vector _asbp_player_test)) (- (.y (Variables|/Game/SaveTheOcean/Enemy/BP_Player_test.BP_Player_test_C|GetPlayer_Vector _asbp_player_test)) 1.3e+02) (.z (Variables|/Game/SaveTheOcean/Enemy/BP_Player_test.BP_Player_test_C|GetPlayer_Vector _asbp_player_test)))))

(fn ConstructionScript)