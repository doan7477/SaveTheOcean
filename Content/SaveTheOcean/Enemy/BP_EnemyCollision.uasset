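; BP_EnemyCollision is a field enemy trigger that sends the player into a battle level.
; When its Box overlaps BP_MovePlayer, it writes the PlayerSpawnSpot world location to the player's PlayerLocation.
; It then saves field info through SaveTheOceanGameInstance and opens the level named by BattleLevelName.
; Debug prints remain in the overlap handler, and the construction script's switch on EnemyName has no case logic.
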(event OnComponentBeginOverlap(Box)
  (params (OverlappedComponent :type Primitive%20Component%20Object%20Reference) (OtherActor :type Actor%20Object%20Reference) (OtherComp :type Primitive%20Component%20Object%20Reference) (OtherBodyIndex :type Integer) (bFromSweep :type Boolean) (SweepResult :type Hit%20Result%20Structure%20%28by%20ref%29))
  ;[1 1 1] Move Player가 맞으면
  (Development|PrintString (Utilities|GetDisplayName OtherActor))
  (bind _asbp_move_player (Utilities|Casting|CastToBP_MovePlayer OtherActor)
    (:then
      (Variables|/Game/SaveTheOcean/Player/Move/BP_MovePlayer.BP_MovePlayer_C|SetPlayerLocation _asbp_move_player (Transformation|GetWorldLocation (Variables|Default|GetPlayerSpawnSpot)))
      ;[1 1 1] 필드 정보를 저장
      (bind _assave_the_ocean_game_instance (Utilities|Casting|CastToSaveTheOceanGameInstance (Game|GetGameInstance)))
      (Default|SaveFieldInfo _assave_the_ocean_game_instance)
      (Game|OpenLevel(byName) (Utilities|String|StringToName (Variables|Default|GetBattleLevelName))))
    (:CastFailed
      (Development|PrintString "Hello"))))

(event EventBeginPlay)

(event Collision|EventActorBeginOverlap
  (params (OtherActor :type Actor%20Object%20Reference)))

(event EventTick
  (params (DeltaSeconds :type Float%20%28single-precision%29)))

(fn ConstructionScript
  (switch Utilities|FlowControl|Switch|SwitchonEnemyName (Variables|Default|GetEnemyName)))